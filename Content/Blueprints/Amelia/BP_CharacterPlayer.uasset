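; Player character Blueprint with movement, camera look, a briefly delayed jump, melee damage and health.
; Axis inputs move the character along control-rotation forward and right vectors and feed controller yaw and pitch.
; MeleeBox overlaps apply fixed damage to actors tagged Enemy, with no attack-state check in this graph.
; Incoming damage reduces Health, but the zero-health branch is empty and a DestroyActor node sits unconnected.
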(event `InputAction|Gangnam`
  (params (Key :type "Key Structure")))

(event `InputAxis|MoveForward`
  (params (AxisValue :type "Float (single-precision)"))
  ;[1 1 1] Movement
  (`self.AddMovementInput` (`KismetMathLibrary.GetForwardVector` (`self.GetControlRotation`)) AxisValue))

(event `InputAxis|MoveRight`
  (params (AxisValue :type "Float (single-precision)"))
  ;[1 1 1] Movement
  (`self.AddMovementInput` (`KismetMathLibrary.GetRightVector` (`self.GetControlRotation`)) AxisValue))

(event `InputAction|Jump`
  (params (Key :type "Key Structure"))
  ;[1 1 1] Movement
  (:`Pressed`
    (`KismetSystemLibrary.Delay` 0.1)
    (`self.Jump`)))

(event `InputAxis|LookUp`
  (params (AxisValue :type "Float (single-precision)"))
  ;[1 1 1] Camera
  (`self.AddControllerPitchInput` AxisValue))

(event `InputAxis|Turn`
  (params (AxisValue :type "Float (single-precision)"))
  ;[1 1 1] Camera
  (`self.AddControllerYawInput` AxisValue))

(event `InputAxis|TurnRate`
  (params (AxisValue :type "Float (single-precision)"))
  ;[1 1 1] Camera
  (`self.AddControllerYawInput` AxisValue))

(event `InputAxis|LookUpRate`
  (params (AxisValue :type "Float (single-precision)"))
  ;[1 1 1] Camera
  (`self.AddControllerPitchInput` AxisValue))

(event `self.MeleeBox.OnComponentBeginOverlap`
  (params (OverlappedComponent :type "PrimitiveComponent Object Reference") (OtherActor :type "Actor Object Reference") (OtherComp :type "PrimitiveComponent Object Reference") (OtherBodyIndex :type Integer) (bFromSweep :type Boolean) (SweepResult :type "HitResult Structure (by ref)"))
  (if (`self.ActorHasTag` OtherActor "Enemy")
    (`GameplayStatics.ApplyDamage` null 20.0 null self "/Script/Engine.DamageType")))

(event `self.ReceiveAnyDamage`
  (params (Damage :type "Float (single-precision)") (DamageType :type "DamageType Object Reference") (InstigatedBy :type "Controller Object Reference") (DamageCauser :type "Actor Object Reference"))
  (set `self.Health` (- (`self.Health`) Damage))
  (if (<= (`self.Health`) 0.0)
    _))

(fn `UserConstructionScript`)