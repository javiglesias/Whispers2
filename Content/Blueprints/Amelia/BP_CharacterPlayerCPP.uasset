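; Player character Blueprint that handles input for jumping, camera reset, an umbrella slash and a Gangnam action.
; Jump fires after a short delay, and Reset Camera plays a timeline that lerps the control rotation toward the CamPositionReference world rotation.
; Umbrella Slash raises IsMeleeAttacking for a fixed window, while the Gangnam flag stays set only as long as its input is held.
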(event `InputAction|Jump`
  (params (Key :type "Key Structure"))
  (:`Pressed`
    (`KismetSystemLibrary.Delay` 0.1)
    (`self.Jump`)))

(event `InputAction|Reset Camera`
  (params (Key :type "Key Structure"))
  (bind _returnvalue (`GameplayStatics.GetPlayerController` 0))
  (:`Pressed`
    (bind (_direction _newtrack_0) (`Timeline|Reset camera transition`)
      (:`Update`
        (`Controller.SetControlRotation` _returnvalue (`KismetMathLibrary.RLerp` (`Controller.GetControlRotation` _returnvalue) (`SceneComponent.K2_GetComponentRotation` (`self.Cam Position Reference`)) _newtrack_0))))))

(event `InputAction|Umbrella Slash`
  (params (Key :type "Key Structure"))
  (:`Pressed`
    (set `self.Is Melee Attacking` true)
    (`KismetSystemLibrary.Delay` 0.8)
    (set `self.Is Melee Attacking` false)))

(event `InputAction|Gangnam`
  (params (Key :type "Key Structure"))
  (:`Pressed`
    (set `self.Gangnam` true))
  (:`Released`
    (set `self.Gangnam` false)))

(fn `UserConstructionScript`)