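; Game mode Blueprint with helper functions for keeping the level populated with AI enemies.
; CheckEnemiesLeft reports whether the live BP_AIEnemy count is below MaxEnemiesCount.
; SpawnMoarEnemies spawns a BP_AIEnemy at a random point inside the given volume's bounds, adjusting for collisions but always spawning.
; Enemy type selection is a stub returning the first EnemiesEnum entry, and no graph here calls the check or spawn.
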(fn `CheckEnemiesLeft`
  (returns (SpawnMoar :type Boolean))
  ;[1 1 1] If there is less enemies that the max, spawn moar.
  (bind _outactors (`GameplayStatics.GetAllActorsOfClass` "/Game/Core/Enemies/BP_AIEnemy.BP_AIEnemy_C"))
  (return (< (`KismetArrayLibrary.Array_Length` _outactors) (`self.MaxEnemiesCount`))))

(fn `ChooseEnemyToSpawn`
  (returns (NewParam :type String))
  (return (`|GetArrayItem` (`self.EnemiesEnum`))))

(fn `SpawnMoarEnemies`
  (params (SpawnVolumeBounds :type "NavMeshBoundsVolume Object Reference"))
  (bind (_origin _boxextent) (`self.GetActorBounds` SpawnVolumeBounds false false))
  ;[1 1 1] Rules to spawn each type of enemy
  (bind _newparam (`self.ChooseEnemyToSpawn`))
  (switch `string` _newparam
    (:`Default`
      _)
    (:`Basic`
      _))
  (`|SpawnActorFromClass` "/Game/Core/Enemies/BP_AIEnemy.BP_AIEnemy_C" (`KismetMathLibrary.MakeTransform` (`KismetMathLibrary.RandomPointInBoundingBox` _origin _boxextent)) "AdjustIfPossibleButAlwaysSpawn" "OverrideRootScale" null null))

(fn `UserConstructionScript`)