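; BP_WaterPuddle is a water puddle that detects the player and is meant to restore their water.
; TriggerIn overlaps set in-puddle flags on puddle and player and notify WaterPuddleManager.
; Entering while needing life or ammo, or calling TakeWaterFromPuddle while occupied, reaches a check on RestoringPlayerWater.
; That branch plays a sound, prints a debug message and starts a timeline, with no life or ammo change wired.
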(event `TakeWaterFromPuddle`
  (if (`self.IsPlayerOnPuddle`)
    (if (`self.RestoringPlayerWater`) :!label _label
      (set `self.RestoringPlayerWater` true)
      (`GameplayStatics.PlaySoundAtLocation` null (0.0 0.0 0.0) (struct) 1.0 1.0 0.0 null null null)
      (`KismetSystemLibrary.PrintString` "HealingPlayer")
      (`Timeline|Timeline_0` :!via `PlayFromStart`))))

(event `self.TriggerIn.OnComponentBeginOverlap`
  (params (OverlappedComponent :type "PrimitiveComponent Object Reference") (OtherActor :type "Actor Object Reference") (OtherComp :type "PrimitiveComponent Object Reference") (OtherBodyIndex :type Integer) (bFromSweep :type Boolean) (SweepResult :type "HitResult Structure (by ref)"))
  (bind _asbp_character_player (cast `/Game/Blueprints/Amelia/BP_CharacterPlayer` OtherActor))
  (set `/Game/Blueprints/Amelia/BP_CharacterPlayer.IsPlayerInPuddle` true _asbp_character_player)
  (set `self.IsPlayerOnPuddle` true)
  (`/Game/Blueprints/Water/BP_WaterPuddleManager.PlayerEnteredPuddle` (`self.WaterPuddleManager`) self)
  ;[1 1 1] Check if character needs water
  (if (or (`/Game/Blueprints/Amelia/BP_CharacterPlayer.PlayerNeedsLife` _asbp_character_player) (`/Game/Blueprints/Amelia/BP_CharacterPlayer.PlayerNeedsAmmo` _asbp_character_player))
    (goto _label)))

(event `self.TriggerIn.OnComponentEndOverlap`
  (params (OverlappedComponent :type "PrimitiveComponent Object Reference") (OtherActor :type "Actor Object Reference") (OtherComp :type "PrimitiveComponent Object Reference") (OtherBodyIndex :type Integer))
  (bind _asbp_character_player (cast `/Game/Blueprints/Amelia/BP_CharacterPlayer` OtherActor))
  (set `/Game/Blueprints/Amelia/BP_CharacterPlayer.IsPlayerInPuddle` false _asbp_character_player)
  (set `self.IsPlayerOnPuddle` false)
  (`/Game/Blueprints/Water/BP_WaterPuddleManager.PlayerLeftPuddle` (`self.WaterPuddleManager`))
  (set `self.RestoringPlayerWater` false))

(fn `UserConstructionScript`)