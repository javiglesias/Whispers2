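; AI enemy character that takes a fixed amount of damage when it collides with the player character.
; BeginPlay writes the Amelia blackboard key through its C++ AI controller, with no object value supplied.
; Each hit briefly disables capsule collision and sets a knockback flag; at zero health it plays an injured animation, then destroys itself.
; Helper functions set walk and sprint speeds; the death-effect logic is disconnected.
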(event `self.ReceiveBeginPlay`
  (bind _ascpp_aicontroller (cast `Cpp_AIController` (`self.GetController` self)))
  (bind _returnvalue (`Cpp_AIController.GeBlackBoardComponent` _ascpp_aicontroller))
  (`BlackboardComponent.SetValueAsObject` _returnvalue (`self.Amelia`) null))

(event `self.ReceiveHit`
  (params (MyComp :type "PrimitiveComponent Object Reference") (Other :type "Actor Object Reference") (OtherComp :type "PrimitiveComponent Object Reference") (bSelfMoved :type Boolean) (HitLocation :type "Vector Structure") (HitNormal :type "Vector Structure") (NormalImpulse :type "Vector Structure") (Hit :type "HitResult Structure (by ref)"))
  (bind _health_0 (`self.Health_0`))
  (bind _capsulecomponent (`self.CapsuleComponent`))
  (cast `/Game/Blueprints/Amelia/BP_CharacterPlayerCPP` Other)
  (if (and (<= 5 _health_0) (not (`self.IsKnockbacked`)))
    (bind _output_get (set `self.Health_0` (- _health_0 5)))
    (if (<= _output_get 0)
      (`PrimitiveComponent.SetCollisionEnabled` _capsulecomponent "NoCollision")
      (`SkeletalMeshComponent.PlayAnimation` (`self.Mesh`) "/Game/Art/Placeholders/Amy/Injured_Hurting_Idle.Injured_Hurting_Idle" false)
      (`KismetSystemLibrary.Delay` 2.5)
      (`self.K2_DestroyActor`)
      (else
        (`PrimitiveComponent.SetCollisionEnabled` _capsulecomponent "NoCollision")
        (set `self.IsKnockbacked` true)
        (`KismetSystemLibrary.Delay` 2.5)
        (set `self.IsKnockbacked` false)
        (`PrimitiveComponent.SetCollisionEnabled` _capsulecomponent "QueryAndPhysics")))))

(event `self.ReceiveDestroyed`
  ;[1 1 1] Effect when enemy die.
)

(fn `SprintSpeed`
  (params (SprintSpeed :type "Float (double-precision)"))
  (set `CharacterMovementComponent.MaxWalkSpeed` SprintSpeed (`self.CharacterMovement`)))

(fn `UserConstructionScript`)

(fn `WalkSpeed`
  (params (WalkSpeed :type "Float (double-precision)"))
  (set `CharacterMovementComponent.MaxWalkSpeed` WalkSpeed (`self.CharacterMovement`)))